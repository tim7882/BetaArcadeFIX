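; Track generator that builds a racetrack along an editable spline in the Construction Script.
; It resizes a per-point road data array toward the spline point count, then loops over segments, optionally closing the circuit.
; Each segment adds spline meshes for track, guard rails, decoration and boost pads, picked by per-point indices and interpolating bank, width and thickness between points.
; Collision is toggleable, and optional text renders number each spline point.
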(fn ConstructionScript
  (Utilities|FlowControl|Sequence
    (:then_0
      (|StoreNumberofSplinePoints))
    (:then_1
      (|BuildRoadDataArray))
    (:then_2
      (|ConstructionLoop)
      (|StoreDrawGuardRails)
      (Utilities|FlowControl|Sequence
        (:then_0
          ;[1 1 1] Draws Track Mesh Type 1
          (CallFunction|BuildTrackElement (Variables|Default|GetCurrentLoopIndex) (Utilities|Array|Get(acopy) (Variables|TrackMeshes|GetTrackArray) (Variables|Default|GetTrackMeshNum))))
        (:then_1
          ;[1 1 1] Draws Left Guard Rail
          (CallFunction|BuildTrackElement (Variables|Default|GetCurrentLoopIndex) (Utilities|Array|Get(acopy) (Variables|TrackMeshes|GetLeftGR_Array) (Variables|Default|GetLGRMeshNum))))
        (:then_2
          ;[1 1 1] Draws Right Guard Rail
          (CallFunction|BuildTrackElement (Variables|Default|GetCurrentLoopIndex) (Utilities|Array|Get(acopy) (Variables|TrackMeshes|GetRightGR_Array) (Variables|Default|GetRGRMeshNum))))
        (:then_3
          ;[1 1 1] Draws Decoration
          (CallFunction|BuildTrackElement (Variables|Default|GetCurrentLoopIndex) (Utilities|Array|Get(acopy) (Variables|TrackMeshes|GetDecoration) (Variables|Default|GetDecMeshNum))))
        (:then_4
          ;[1 1 1] Builds Boost Pads
          (CallFunction|BuildTrackElement (Variables|Default|GetCurrentLoopIndex) (Utilities|Array|Get(acopy) (Variables|TrackMeshes|GetBoostPads) (Variables|Default|GetBoostMeshNum))))))
    (:then_3
      (|DrawTrackPointNumbers))))

(fn BuildTrackElement
  (params (LoopIndex :type Integer) (TrackElementMesh :type Static%20Mesh%20Object%20Reference))
  (LocalVariables|SetLocal_CurrentLoopIndex LoopIndex)
  (LocalVariables|SetLocal_NextLoopIndex (Math|Integer|%(Integer) (+ LoopIndex 1) (Variables|Default|GetNumberofSplinePoints)))
  (LocalVariables|SetLocal_TrackElementMesh TrackElementMesh)
  (Utilities|FlowControl|Sequence
    (:then_0
      (LocalVariables|SetLocal_StartLocation (.Location (Spline|GetLocationandTangentatSplinePoint (Variables|Default|GetSpline) (LocalVariables|GetLocal_CurrentLoopIndex) "Local")))
      (LocalVariables|SetLocal_StartTangent (.Tangent (Spline|GetLocationandTangentatSplinePoint (Variables|Default|GetSpline) (LocalVariables|GetLocal_CurrentLoopIndex) "Local")))
      (LocalVariables|SetLocal_EndLocation (.Location (Spline|GetLocationandTangentatSplinePoint (Variables|Default|GetSpline) (LocalVariables|GetLocal_NextLoopIndex) "Local")))
      (LocalVariables|SetLocal_EndTangent (.Tangent (Spline|GetLocationandTangentatSplinePoint (Variables|Default|GetSpline) (LocalVariables|GetLocal_NextLoopIndex) "Local")))
      (LocalVariables|SetLocal_StartRoll (.trackbank (Utilities|Array|Get(acopy) (Variables|TrackSetUp|GetRoadDataArray) (LocalVariables|GetLocal_CurrentLoopIndex))))
      (LocalVariables|SetLocal_StartScale (Math|Vector2D|MakeVector2D (.trackwidth (Utilities|Array|Get(acopy) (Variables|TrackSetUp|GetRoadDataArray) (LocalVariables|GetLocal_CurrentLoopIndex))) (.trackthickness (Utilities|Array|Get(acopy) (Variables|TrackSetUp|GetRoadDataArray) (LocalVariables|GetLocal_CurrentLoopIndex)))))
      (LocalVariables|SetLocal_EndRoll (.trackbank (Utilities|Array|Get(acopy) (Variables|TrackSetUp|GetRoadDataArray) (LocalVariables|GetLocal_NextLoopIndex))))
      (LocalVariables|SetLocal_EndScale (Math|Vector2D|MakeVector2D (.trackwidth (Utilities|Array|Get(acopy) (Variables|TrackSetUp|GetRoadDataArray) (LocalVariables|GetLocal_NextLoopIndex))) (.trackthickness (Utilities|Array|Get(acopy) (Variables|TrackSetUp|GetRoadDataArray) (LocalVariables|GetLocal_NextLoopIndex))))))
    (:then_1
      (bind _returnvalue (AddComponent|AddSplineMeshComponent false))
      (LocalVariables|SetLocal_CurrentSplineMesh _returnvalue)
      (Components|StaticMesh|SetStaticMesh (LocalVariables|GetLocal_CurrentSplineMesh) (LocalVariables|GetLocal_TrackElementMesh))
      (SplineMesh|SetStartandEnd (LocalVariables|GetLocal_CurrentSplineMesh) (LocalVariables|GetLocal_StartLocation) (LocalVariables|GetLocal_StartTangent) (LocalVariables|GetLocal_EndLocation) (LocalVariables|GetLocal_EndTangent) true :!class /Script/Engine.SplineMeshComponent)
      (Class|SplineMeshComponent|SetStartRoll (LocalVariables|GetLocal_CurrentSplineMesh) (LocalVariables|GetLocal_StartRoll) true)
      (Class|SplineMeshComponent|SetEndRoll (LocalVariables|GetLocal_CurrentSplineMesh) (LocalVariables|GetLocal_EndRoll) true)
      (SplineMesh|SetStartScale (LocalVariables|GetLocal_CurrentSplineMesh) (LocalVariables|GetLocal_StartScale) true :!class /Script/Engine.SplineMeshComponent)
      (SplineMesh|SetEndScale (LocalVariables|GetLocal_CurrentSplineMesh) (LocalVariables|GetLocal_EndScale) true :!class /Script/Engine.SplineMeshComponent)
      (Collision|SetCollisionEnabled (LocalVariables|GetLocal_CurrentSplineMesh) (select (Variables|Debug|GetCollisions) "QueryAndPhysics" "NoCollision")))))