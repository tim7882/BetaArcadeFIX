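; Boost pad actor that speeds up a Sedan vehicle when it drives over it.
; On overlap, a Duration timeline drives the Speed variable of the Sedan cached at BeginPlay, not necessarily the overlapping one.
; The overlapping Sedan's mesh also has its physics velocity replaced with a fixed push along the pad's negative right vector.
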(event EventBeginPlay
  (bind _returnvalue (Actor|GetActorOfClass "/Game/tim/player/Sedan.Sedan_C"))
  (Variables|Default|SetSedan _returnvalue))

(event Collision|EventActorBeginOverlap
  (params (OtherActor :type Actor%20Object%20Reference))
  (Utilities|FlowControl|Sequence
    (:then_0
      (bind _assedan (Utilities|Casting|CastToSedan OtherActor))
      (bind _newtrack_0 (Timeline|Duration Play)
        (:Update
          (Variables|/Game/tim/player/Sedan.Sedan_C|SetSpeed (Variables|Default|GetSedan) _newtrack_0))))
    (:then_1
      (bind _assedan_2 (Utilities|Casting|CastToSedan OtherActor))
      (Physics|SetPhysicsLinearVelocity (Variables|/Script/PhysXVehicles.WheeledVehicle|GetMesh _assedan_2) (* (Transformation|GetActorRightVector) -7.5e+02) false "None"))))

(event EventTick
  (params (DeltaSeconds :type Float%20%28single-precision%29)))

(fn ConstructionScript)